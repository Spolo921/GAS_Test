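; Gameplay ability that equips or unequips the avatar's weapon when activated by a gameplay event.
; It commits, then switches on the event's first target tag and calls the avatar's Weapons Manager component.
; The two secondary pistol tags equip their matching pistol Blueprint, while any other tag unequips the current weapon.
; The ability ends right after that call, provided the component is valid.
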(event Ability|EventActivateAbilityFromEvent
  (params (EventData :type Gameplay%20Event%20Data%20Structure%20%28by%20ref%29))
  (bind _returnvalue (Ability|GetAvatarActorfromActorInfo))
  (bind _returnvalue_2 (Actor|GetComponentbyClass _returnvalue "/Game/Weapons/Weapons_Manager_Component.Weapons_Manager_Component_C"))
  (Ability|CommitAbility)
  (Utilities|IsValid _returnvalue_2
    (:Is%20Valid
      (Utilities|FlowControl|Sequence
        (:then_0
          (|SwitchGameplayTag (Utilities|Array|Get(acopy) (GameplayTags|BreakGameplayTagContainer (.TargetTags (Utilities|Struct|BreakGameplayEventData EventData))))
            (:Default
              (Default|UnequipWeapon _returnvalue_2))
            (:Weapon.Secondary.Pistol1
              (Default|EquipWeapon _returnvalue_2 "/Game/Weapons/BP_Pistol1.BP_Pistol1_C"))
            (:Weapon.Secondary.Pistol2
              (Default|EquipWeapon _returnvalue_2 "/Game/Weapons/BP_Pistol2.BP_Pistol2_C"))))
        (:then_1
          (Ability|EndAbility))))))